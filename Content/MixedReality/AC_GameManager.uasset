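; Game manager component that takes the mixed-reality game from launch to play.
; It checks or requests Android storage and Quest scene permissions, then spawns a menu display at the camera.
; When the safety-screen timer completes, it removes the menu, signals room-data spawning, switches streaming levels and starts music.
; It then spawns the interior from MRUK room anchors and a pistol at the table anchor, falling back to the floor.
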(event Custom|PermissionsGrantedResult
  (params (Permissions :type Array%20of%20Strings) (GrantResults :type Array%20of%20Booleans))
  (if (== (Utilities|Array|Length GrantResults) 3)
    (Development|PrintString " 
 
 
 
 
 
All Permissions are Granted")
    (Utilities|FlowControl|Delay 1.0)
    (CallFunction|SpawnMainMenu)
    (else
      (Development|PrintString " 
 
 
 
 
 
 
Failed to request all Permissions"))))

(event Custom|SpawnMainMenu
  (bind _returnvalue (Game|GetPlayerCameraManager 0))
  (bind _rootcomponent (Variables|/Script/Engine.Actor|GetRootComponent _returnvalue))
  ;[1 1 1] Spawn Main Menu Actor
  (bind _returnvalue_2 (Game|SpawnActorfromClass "/Game/MixedReality/Widgets/BP_UMGDisplay.BP_UMGDisplay_C" (Math|Transform|MakeTransform (Transformation|GetWorldLocation _rootcomponent) (Transformation|GetWorldRotation _rootcomponent) "1.000000,1.000000,1.000000") "Undefined" "MultiplyWithRoot" 0 0))
  (bind _output_get (Variables|Default|SetSpawned%20UMG%20Actor _returnvalue_2))
  ;[1 1 1] Get Safety Screen and Listen to Timer is Complete
  (Default|CallSpawnedMainMenu)
  (bind _aswbp_main_menu (Utilities|Casting|CastToWBP_MainMenu (UserInterface|GetWidget (Variables|/Game/MixedReality/Widgets/BP_UMGDisplay.BP_UMGDisplay_C|GetWidget _output_get))))
  (EventDispatchers|BindEventtoTimerComplete (Variables|/Game/MixedReality/Widgets/WBP_MainMenu.WBP_MainMenu_C|GetWBP_SafetyScreen _aswbp_main_menu) (delegate Custom|TimerComplete_Event)))

(event Custom|TimerComplete_Event
  ;[1 1 1] If timer is complete, destroy menu and start the game
  (Actor|DestroyActor (stale Custom|SpawnMainMenu _output_get))
  (Variables|Default|SetSpawned%20UMG%20Actor 0)
  (Default|CallSpawnRoomData)
  (CallFunction|SpawnRoomInterior))

(event Custom|SpawnRoomInterior
  (Audio|PlaySound2D "/Game/MixedReality/Audio/perfect-beauty-music.perfect-beauty-music" 0.7 1.0 0.0 0 0)
  (Variables|/Script/Engine.LevelStreaming|SetbShouldBeVisible (Class|GameplayStatics|GetStreamingLevel "OutsideEnvironment") true)
  (Variables|/Script/Engine.LevelStreaming|SetbShouldBeVisible (Class|GameplayStatics|GetStreamingLevel "MenuLighting") false)
  ;[1 1 1] Spawn Interior from our MRUK
  (bind _returnvalue (Actor|GetActorOfClass "/Script/MRUtilityKit.MRUKAnchorActorSpawner"))
  (Class|MRUKAnchorActorSpawner|SpawnActors _returnvalue (Class|MRUKSubsystem|GetCurrentRoom (Subsystems|GetMRUKSubsystem)))
  (Default|CallSpawnedInterior)
  (CallFunction|SpawnPlayerWeapons))

(event Custom|Spawn%20Player%20Weapons
  (bind _returnvalue (Subsystems|GetMRUKSubsystem))
  (bind _returnvalue_2 (Class|MRUKSubsystem|GetCurrentRoom _returnvalue))
  (bind _returnvalue_3 (Class|MRUKRoom|GetAnchorsbyLabel _returnvalue_2 "TABLE"))
  (bind _output (Utilities|Array|Get(acopy) _returnvalue_3))
  ;[1 1 1] Spawn Actors using Room Anchors (need to load room data from device async before)
  (if (Utilities|IsValid _output)
    (Variables|Default|SetWeaponSpawnLocation (Transformation|GetActorLocation _output))
    (else
      (Variables|Default|SetWeaponSpawnLocation (Transformation|GetActorLocation (Utilities|Array|Get(acopy) (Class|MRUKRoom|GetAnchorsbyLabel _returnvalue_2 "FLOOR"))))))
  (Game|SpawnActorfromClass "/Game/VRTemplate/Blueprints/Pistol.Pistol_C" (Math|Transform|MakeTransform (Variables|Default|GetWeaponSpawnLocation) "0, 0, 0" "1.000000,1.000000,1.000000") "Undefined" "MultiplyWithRoot" 0 0))

(event EventBeginPlay
  (bind _array (Utilities|Array|MakeArray "android.permission.WRITE_EXTERNAL_STORAGE" "android.permission.READ_EXTERNAL_STORAGE" "com.oculus.permission.USE_SCENE"))
  (for (_array_element _array_index) _array
    (bind _returnvalue (Class|AndroidPermissionFunctionLibrary|CheckPermission _array_element))
    (if _returnvalue
      (bind _returnvalue_2 (Utilities|Array|Add (Variables|Default|GetNumberOfPermissions) _array_index))
      (if (== _returnvalue_2 2)
        (Development|PrintString " 
 
 
 
 
 
All Permissions are Granted")
        (Utilities|FlowControl|Delay 1.0)
        (CallFunction|SpawnMainMenu)
        (else
          (Development|PrintString " 
 
 
 
 
 
 
Failed to request all Permissions")))
      (else
        (bind _returnvalue_3 (Class|AndroidPermissionFunctionLibrary|AcquirePermissions _array))
        (EventDispatchers|BindEventtoOnPermissionsGrantedDynamicDelegate _returnvalue_3 (delegate Custom|PermissionsGrantedResult))))))